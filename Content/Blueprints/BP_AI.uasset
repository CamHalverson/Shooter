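; Enemy AI character with a rifle that wanders, chases seen pawns and fires on them.
; A looping BeginPlay repeatedly starts random roaming and clears the seen flag, while PawnSensing sightings trigger a chase that fires on arrival.
; Firing plays a montage whose notify runs a muzzle-socket line trace for damage, effects and sound.
; Damage lowers health to ragdoll death, and Tick updates a camera-facing health bar.
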(event `self.ReceiveBeginPlay`
  (`self.Search Around` :!label _label)
  (`KismetSystemLibrary.Delay` 1.0)
  (`self.Search Around`)
  (set `self.hasSeenTarget?` false)
  (goto _label))

(event `Search Around`
  ;[1 1 1] Search Around
  (if (not (`self.hasSeenTarget?`))
    (`|AIMoveTo` self (`NavigationSystemV1.K2_GetRandomReachablePointInRadius` (`self.K2_GetActorLocation`) 2000.0 null null) null 450.0
      (:`OnSuccess`
        (`KismetSystemLibrary.Delay` 1.0)
        (`self.Search Around`)))))

(event `self.ReceiveAnyDamage`
  (params (Damage :type "Float (single-precision)") (DamageType :type "DamageType Object Reference") (InstigatedBy :type "Controller Object Reference") (DamageCauser :type "Actor Object Reference"))
  ;[1 1 1] Health
  (set `self.health` (- (`self.health`) Damage))
  (if (<= (`self.health`) 0.0)
    (`KismetSystemLibrary.PrintString` "Die")
    (`PrimitiveComponent.SetSimulatePhysics` (`self.Mesh`) true)
    (`CharacterMovementComponent.SetMovementMode` (`self.CharacterMovement`) "MOVE_None" 0)
    (set `self.isDead?` true)
    (`SceneComponent.SetVisibility` (`self.Healthbar Widget`) false false)
    (else
      (`KismetSystemLibrary.PrintString` "Damage"))))

(event `self.PawnSensing.OnSeePawn`
  (params (Pawn :type "Pawn Object Reference"))
  (`self.Chase Target` Pawn)
  (set `self.hasSeenTarget?` true))

(event `Chase Target`
  (params (TargetActor :type "Actor Object Reference"))
  (`|AIMoveTo` self (0.0 0.0 0.0) TargetActor 300.0
    (:`OnSuccess`
      (`self.Fire` TargetActor))))

(event `Fire`
  (params (`Target Actor` :type "Actor Object Reference"))
  (bind _returnvalue_location (`KismetMathLibrary.BreakTransform` (`SceneComponent.GetSocketTransform` (`self.Rifle`) "b_gun_muzzleflash" "RTS_World")))
  (bind _returnvalue (`SceneComponent.K2_GetComponentRotation` (`self.Mesh`)))
  (if (not (`self.isDead?`))
    (`Controller.SetControlRotation` (`self.GetController`) (`KismetMathLibrary.FindLookAtRotation` (`self.K2_GetActorLocation`) (`self.K2_GetActorLocation` `Target Actor`)))
    (`|PlayMontage` (`self.Mesh`) "/Game/ShooterAnim/Fire_Montage.Fire_Montage"
      (:`OnNotifyBegin`
        (`GameplayStatics.SpawnEmitterAttached` "/Game/InfinityBladeEffects/Effects/FX_Monsters/FX_Monster_Gruntling/Master/P_BackPack_MuzzleFlash.P_BackPack_MuzzleFlash" (`self.Rifle`) "b_gun_muzzleflash" _returnvalue_location _returnvalue (0.2 0.2 0.2) "KeepWorldPosition" true "AutoRelease")
        (`GameplayStatics.PlaySoundAtLocation` "/Game/Audio/MS_Rifle_Fire.MS_Rifle_Fire" (`self.K2_GetActorLocation`) (struct) 0.6 1.0 0.0 null null null null)
        (bind (_outhit _returnvalue_2) (`KismetSystemLibrary.LineTraceSingle` _returnvalue_location (+ _returnvalue_location (* (`KismetMathLibrary.GetRightVector` _returnvalue) 3000.0)) "TraceTypeQuery1"))
        (if _returnvalue_2
          (bind (_bblockinghit _binitialoverlap _time _distance _location _impactpoint _normal _impactnormal _physmat _hitactor) (`GameplayStatics.BreakHitResult` _outhit))
          (`GameplayStatics.ApplyDamage` _hitactor 5.0)
          (`GameplayStatics.SpawnEmitterAtLocation` "/Game/InfinityBladeEffects/Effects/FX_Monsters/FX_Monster_Troll/death/P_TrollDeathImpact.P_TrollDeathImpact" _impactpoint (`KismetMathLibrary.MakeRotFromX` _normal) (0.6 0.6 0.6) true "AutoRelease"))))))

(event `self.ReceiveTick`
  (params (DeltaSeconds :type "Float (single-precision)"))
  (bind _aswb_ai_healthbar (cast `/Game/WB_AI_Healthbar` (`WidgetComponent.GetWidget` (`self.Healthbar Widget`))))
  (`ProgressBar.SetPercent` (`/Game/WB_AI_Healthbar.Healthbar` _aswb_ai_healthbar) (/ (`self.health`) 100.0))
  (`SceneComponent.K2_SetWorldRotation` (`self.Healthbar Widget`) (`KismetMathLibrary.FindLookAtRotation` (`self.K2_GetActorLocation`) (`self.K2_GetActorLocation` (`GameplayStatics.GetPlayerCameraManager` 0))) false false))

(fn `UserConstructionScript`)