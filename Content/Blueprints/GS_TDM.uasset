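; GS_TDM is the team deathmatch state Blueprint, tracking how many players remain alive on Team A and Team B.
; DecreaseTeamNumber decrements the count for the team chosen by its boolean and, when that reaches zero, shows a WB_TeamWinner widget naming the other team.
; Otherwise UpdateWidget writes both counts to the player 0 character's HUD, as it also does shortly after BeginPlay.
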(event `self.ReceiveBeginPlay`
  (`KismetSystemLibrary.Delay` 0.2)
  (`self.Update Widget`))

(event `Decrease Team Number`
  (params (Condition :type Boolean))
  (if Condition
    (bind _result (`/Engine/EditorBlueprintResources/StandardMacros.DecrementInt` (`self.NumOfTeamA_Alive`))
      (:`  `
        (if (<= _result 0)
          (bind _returnvalue (`|CreateWidget` "/Game/WB_TeamWinner.WB_TeamWinner_C"))
          (`TextBlock.SetText` (`/Game/WB_TeamWinner.WinnerText` _returnvalue) "TEAM B WON")
          (`UserWidget.AddToViewport` _returnvalue 0)
          (else
            (`self.Update Widget` :!label _label)))))
    (else
      (bind _result_2 (`/Engine/EditorBlueprintResources/StandardMacros.DecrementInt` (`self.NumOfTeamB_Alive`))
        (:`  `
          (if (<= _result_2 0)
            (bind _returnvalue_2 (`|CreateWidget` "/Game/WB_TeamWinner.WB_TeamWinner_C"))
            (`TextBlock.SetText` (`/Game/WB_TeamWinner.WinnerText` _returnvalue_2) "TEAM A WON")
            (`UserWidget.AddToViewport` _returnvalue_2 0)
            (else
              (goto _label))))))))

(event `Update Widget`
  (bind _asbp_third_person_character (cast `/Game/ThirdPerson/Blueprints/BP_ThirdPersonCharacter` (`GameplayStatics.GetPlayerCharacter` 0)))
  (bind _hud (`/Game/ThirdPerson/Blueprints/BP_ThirdPersonCharacter.HUD` _asbp_third_person_character))
  (`TextBlock.SetText` (`/Game/WB_Hud.TeamAtext` _hud) (`|FormatText` "Team A: {Value}" (`self.NumOfTeamA_Alive`)))
  (`TextBlock.SetText` (`/Game/WB_Hud.TeamBtext` _hud) (`|FormatText` "Team B: {Value}" (`self.NumOfTeamB_Alive`))))

(fn `UserConstructionScript`)